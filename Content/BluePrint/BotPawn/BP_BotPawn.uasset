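; BP_BotPawn is a player-controllable bot pawn with mouse-look style aiming and twin rifles that fire alternately.
; On BeginPlay it adds the bot's Enhanced Input mapping context, and look input drives controller yaw and pitch.
; Each fire input toggles a FlipFlop that tells FireRifle whether to use the left or right mesh socket.
; FireRifle spawns an actor at that socket with a beam burst effect and an energy rifle sound.
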(event `self.ReceiveBeginPlay`
  ;[0.15 0.04977 0.01964 0.5] Add Bot Mapping Context
  (bind _asplayer_controller (cast `PlayerController` (`self.GetController`)))
  (`EnhancedInputSubsystemInterface.AddMappingContext` (pcsubsystem `EnhancedInputLocalPlayerSubsystem` _asplayer_controller) "/Game/BluePrint/Input/IMCBot.IMCBot" 0 (struct)))

(event `EnhancedInput|/Game/BluePrint/Input/InputActions/IA_Fire`
  (params (ActionValue :type Boolean) (ElapsedSeconds :type "Float (double-precision)") (TriggeredSeconds :type "Float (double-precision)") (InputAction :type "InputAction Object Reference" :default "/Game/BluePrint/Input/InputActions/IA_Fire.IA_Fire"))
  (:`Triggered`
    (bind _isa (`/Engine/EditorBlueprintResources/StandardMacros.FlipFlop`)
      (:`A`
        _)
      (:`B`
        _))
    (`self.FireRifle` _isa)))

(event `EnhancedInput|/Game/BluePrint/Input/InputActions/IA_Look`
  (params (ActionValue :type "Vector2D Structure") (ElapsedSeconds :type "Float (double-precision)") (TriggeredSeconds :type "Float (double-precision)") (InputAction :type "InputAction Object Reference" :default "/Game/BluePrint/Input/InputActions/IA_Look.IA_Look"))
  (bind (_x _y) (`KismetMathLibrary.BreakVector2D` ActionValue))
  (:`Triggered`
    (`self.AddControllerYawInput` _x)
    (`self.AddControllerPitchInput` _y)))

(fn `FireRifle`
  (params (IsLeftRifle :type Boolean))
  (bind (_returnvalue_location _returnvalue_rotation) (`KismetMathLibrary.BreakTransform` (`SceneComponent.GetSocketTransform` (`self.BotMesh`) (`self.SocketName`) "RTS_World")))
  (if IsLeftRifle
    (set `self.SocketName` "Rifle_L")
    (else
      (set `self.SocketName` "Rifle_R")))
  (`|SpawnActorFromClass` "/Game/BluePrint/BlasterBeam/BP_BlasterBeam.BP_BlasterBeam_C" (`SceneComponent.GetSocketTransform` (`self.BotMesh`) (`self.SocketName`) "RTS_World") "Undefined" "MultiplyWithRoot" null null null)
  (`NiagaraFunctionLibrary.SpawnSystemAtLocation` "/Game/Assets/FX/NS_BeamBurst.NS_BeamBurst" _returnvalue_location _returnvalue_rotation)
  (`GameplayStatics.PlaySoundAtLocation` "/Game/Assets/Sounds/Drone/sfx_EnergyRifle.sfx_EnergyRifle" _returnvalue_location (struct) 1.0 1.0 0.0 null null null null))

(fn `UserConstructionScript`)