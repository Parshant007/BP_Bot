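; BP_SmallSphere is a short-lived moving pickup sphere that increments the score in BP_BadBotGameMode when a Pawn overlaps it.
; After a short delay on BeginPlay it scales in, picks a random spin, starts a lifetime timer and binds the overlap.
; Tick moves it along its rotating forward vector, so it wanders.
; Overlap or timer expiry triggers a guarded WinkOut timeline that shrinks the mesh and destroys the actor.
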(event `self.ReceiveBeginPlay`
  (`KismetSystemLibrary.Delay` 2.0)
  (`self.WinkIn`)
  ;[0.15 0.06759 0.03581 0.5] Start WinkOut Timeline
  (`self.InitanlizeDeltaRotation`)
  (`KismetSystemLibrary.K2_SetTimerDelegate` (delegate `WinkOut`) (`self.LifeTime`))
  ;[0.15 0 0 0.5] Handl Overlap
  (add `PrimitiveComponent.OnComponentBeginOverlap` (`self.SphereVolume`) (delegate `OnSphereOverlap`)))

(event `OnSphereOverlap`
  (params (OverlappedComponent :type "PrimitiveComponent Object Reference") (OtherActor :type "Actor Object Reference") (OtherComp :type "PrimitiveComponent Object Reference") (OtherBodyIndex :type Integer) (bFromSweep :type Boolean) (SweepResult :type "HitResult Structure (by ref)"))
  ;[0.15 0.06759 0.03581 0.5] Start WinkOut Timeline
  ;[0.15 0 0 0.5] Handl Overlap
  (if (`GameplayStatics.ObjectIsA` OtherActor "/Script/Engine.Pawn")
    (bind _asbp_bad_bot_game_mode (cast `/Game/BluePrint/Game/BP_BadBotGameMode` (`GameplayStatics.GetGameMode`)))
    (`/Game/BluePrint/Game/BP_BadBotGameMode.IncrementScore` _asbp_bad_bot_game_mode)
    (`self.WinkOut`)))

(event `WinkOut`
  ;[0.15 0.06759 0.03581 0.5] Start WinkOut Timeline
  (if (not (`self.IsWinking`))
    (set `self.IsWinking` true)
    (bind (_direction _scale) (`Timeline|WinkOutTimeLine`)
      (:`Update`
        (`self.ScaleSphere` _scale))
      (:`Finished`
        (`self.K2_DestroyActor`)))))

(event `self.ReceiveTick`
  (params (DeltaSeconds :type "Float (single-precision)"))
  ;[0.1064 0.15 0.06869 0.5] Update Location and Rotation
  (`self.UpdateLocation` DeltaSeconds)
  (`self.UpdateRotation` DeltaSeconds))

(event `WinkIn`
  (bind (_direction _scale) (`Timeline|WinkInTimeLine`)
    (:`Update`
      (`SceneComponent.SetWorldScale3D` (`self.SphereMesh`) _scale))))

(fn `InitanlizeDeltaRotation`
  (set `self.Delta Rotation` (* (`KismetMathLibrary.RandomRotator` false) (`self.RotationScaleFactor`))))

(fn `ScaleSphere`
  (params (Scale :type "Float (single-precision)"))
  (`SceneComponent.SetWorldScale3D` (`self.SphereMesh`) (`KismetMathLibrary.MakeVector` Scale Scale Scale)))

(fn `UpdateLocation`
  (params (DeltaSeconds :type "Float (double-precision)"))
  (`self.K2_AddActorWorldOffset` (* (`self.GetActorForwardVector`) (* DeltaSeconds (`self.Speed`)))))

(fn `UpdateRotation`
  (params (DeltaSeconds :type "Float (single-precision)"))
  (`self.K2_AddActorWorldRotation` (* (`self.Delta Rotation`) DeltaSeconds)))

(fn `UserConstructionScript`)