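; BP_SphereSpawner is an actor that periodically spawns BP_SmallSphere actors at random points around itself.
; BeginPlay starts a looping timer at SpawnTime intervals, and each tick spawns one sphere with a random rotation.
; GetRandomPointsSphereRadius picks the location by offsetting the spawner along a random direction by a random distance up to SpawnRadius.
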(event `self.ReceiveBeginPlay`
  ;[0.15 0 0 0.5] Start Spawn Timer
  (`KismetSystemLibrary.K2_SetTimerDelegate` (delegate `SpawnSmallSphere`) (`self.SpawnTime`) true))

(event `SpawnSmallSphere`
  ;[0.15 0 0 0.5] Start Spawn Timer
  (`|SpawnActorFromClass` "/Game/BluePrint/SmallSphere/BP_SmallSphere.BP_SmallSphere_C" (`KismetMathLibrary.MakeTransform` (`self.GetRandomPointsSphereRadius`) (`KismetMathLibrary.RandomRotator` false)) "Undefined" "MultiplyWithRoot" null null))

(fn `GetRandomPointsSphereRadius`
  (returns (RandomPoints :type "Vector Structure"))
  (return (+ (`self.K2_GetActorLocation`) (* (`KismetMathLibrary.GetForwardVector` (`KismetMathLibrary.RandomRotator` false)) (`KismetMathLibrary.RandomFloatInRange` 0.0 (`self.SpawnRadius`))))))

(fn `UserConstructionScript`)